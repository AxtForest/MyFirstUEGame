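; BP_Enemy is a melee enemy that chases the player and knocks characters back.
; Pawn sensing triggers an AI move to the player; on arrival it plays an attack montage if allowed.
; As the montage starts, a debug-drawn sphere trace launches any hit Character along the enemy's forward vector, though its endpoint multiplies location by direction instead of adding.
; A montage notify or interruption re-enables attacking.
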(event OnSeePawn(PawnSensing)
  (params (Pawn :type Pawn%20Object%20Reference))
  (CallFunction|ChasePlayer))

(event Custom|ChasePlayer
  (bind _returnvalue (Transformation|GetActorLocation))
  (AI|AIMoveTo self "0, 0, 0" (Game|GetPlayerCharacter 0) 1.2e+02 false
    (:OnSuccess
      (if (Variables|Default|GetCanAttack)
        (Animation|Montage|PlayMontage (Variables|Character|GetMesh) "/Game/Characters/Villager/Animations/AttackMontage.AttackMontage"
          (:then
            (Variables|Default|SetCanAttack false)
            (bind (_outhit _returnvalue_2) (Collision|SphereTraceByChannel _returnvalue (* _returnvalue (* (Math|Vector|GetForwardVector (Transformation|GetActorRotation)) 1.8e+02)) 25.0 "TraceTypeQuery3" false 0 "ForDuration" true "(R=1.000000,G=0.000000,B=0.000000,A=1.000000)" "(R=0.000000,G=1.000000,B=0.000000,A=1.000000)" 0.5))
            (if _returnvalue_2
              (bind _ascharacter (Utilities|Casting|CastToCharacter (.HitActor (Collision|BreakHitResult _outhit))))
              (Character|LaunchCharacter _ascharacter (* (* (Math|Vector|GetForwardVector (Transformation|GetActorRotation)) (Variables|Default|GetFrontalKnockback)) (Variables|Default|GetUpgradeKnockback)) false false)))
          (:OnInterrupted
            (Variables|Default|SetCanAttack true :!label _label))
          (:OnNotifyBegin
            (goto _label)))))))

(event EventBeginPlay)

(fn ConstructionScript)